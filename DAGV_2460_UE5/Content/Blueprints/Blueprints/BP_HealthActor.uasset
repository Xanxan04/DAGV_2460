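; BP_HealthActor is a trigger actor that either damages or heals the third-person player character on contact.
; When its sphere begins overlapping a BP_ThirdPersonCharacter, an ActorType switch selects whether to subtract or add FloatValue.
; The result is clamped to a hardcoded range and written directly to Health on the character's ACCharacterStats component, and the actor stays in place afterward.
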(event OnComponentBeginOverlap(Sphere)
  (params (OverlappedComponent :type Primitive%20Component%20Object%20Reference) (OtherActor :type Actor%20Object%20Reference) (OtherComp :type Primitive%20Component%20Object%20Reference) (OtherBodyIndex :type Integer) (bFromSweep :type Boolean) (SweepResult :type Hit%20Result%20Structure%20%28by%20ref%29))
  (bind _floatvalue (Variables|Default|GetFloatValue))
  (bind _asbp_third_person_character (Utilities|Casting|CastToBP_ThirdPersonCharacter OtherActor))
  (switch Utilities|FlowControl|Switch|SwitchonE_DamageHealing (Variables|Default|GetActorType)
    (:NewEnumerator0
      (Variables|/Game/Blueprints/Blueprints/ActorComponents/AC_CharacterStats.AC_CharacterStats_C|SetHealth (Variables|/Game/ThirdPerson/Blueprints/BP_ThirdPersonCharacter.BP_ThirdPersonCharacter_C|GetAC_CharacterStats _asbp_third_person_character) (Math|Float|Clamp(Float) (- (Variables|/Game/Blueprints/Blueprints/ActorComponents/AC_CharacterStats.AC_CharacterStats_C|GetHealth (Variables|/Game/ThirdPerson/Blueprints/BP_ThirdPersonCharacter.BP_ThirdPersonCharacter_C|GetAC_CharacterStats _asbp_third_person_character)) _floatvalue) 0.0 1e+02)))
    (:NewEnumerator1
      (Variables|/Game/Blueprints/Blueprints/ActorComponents/AC_CharacterStats.AC_CharacterStats_C|SetHealth (Variables|/Game/ThirdPerson/Blueprints/BP_ThirdPersonCharacter.BP_ThirdPersonCharacter_C|GetAC_CharacterStats _asbp_third_person_character) (Math|Float|Clamp(Float) (+ (Variables|/Game/Blueprints/Blueprints/ActorComponents/AC_CharacterStats.AC_CharacterStats_C|GetHealth (Variables|/Game/ThirdPerson/Blueprints/BP_ThirdPersonCharacter.BP_ThirdPersonCharacter_C|GetAC_CharacterStats _asbp_third_person_character)) _floatvalue) 0.0 1e+02)))))

(fn ConstructionScript)