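; Game instance for a falling-object matching game that handles the start countdown, score and high score, and reset.
; Init unpossesses the player and counts down, firing update and finished events.
; While the game state is active, a delay loop spawns fall actors at random fall points and adjusts directional light intensity.
; A one-second timer shortens the spawn delay as play time grows, using a negative-exponent power curve.
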(event Custom|OnScoreUpdate_Event
  (params (ScoreAdd :type Float%20%28double-precision%29))
  (Audio|PlaySound2D "/Game/Media/SFX/Score.Score" 1.0 1.0 0.0 0 0)
  (bind _output_get (Variables|Default|SetScore (+ ScoreAdd (Variables|Default|GetScore))))
  (if (> _output_get (Variables|Default|GetHighScore))
    (Variables|Default|SetHighScore (Variables|Default|GetScore))))

(event Custom|OnReset_Event
  (Variables|Default|SetScore 0.0)
  (Default|CallOnReset)
  (bind _returnvalue (Actor|GetActorOfClass "/Game/ThirdPerson/Blueprints/BP_ThirdPersonCharacter.BP_ThirdPersonCharacter_C"))
  (Input|DisableInput _returnvalue (Game|GetPlayerController 0))
  (Audio|PlaySound2D "/Game/Media/SFX/Shutdown.Shutdown" 1.0 1.0 0.0 0 0)
  (Actor|DestroyActor _returnvalue)
  (Variables|Default|SetGameState false))

(event Custom|InGameTimer
  (bind _result (Math|Float|IncrementFloat (Variables|Default|GetInGameSeconds))
    (:%20%20
      (bind _output_get (Variables|Default|SetSpawnSpeed (Math|Float|Power _result -0.05)))
      (Development|PrintString (Utilities|String|ToString(Float) _output_get)))))

(event Custom|OnFinishedCountdown_Event
  (bind _outactors (Actor|GetAllActorsOfClass "/Game/Blueprints/Blueprints/BP_FallPoint.BP_FallPoint_C"))
  (Variables|Default|SetFallSpawnPoints _outactors)
  (bind _returnvalue (Actor|GetActorOfClass "/Script/Engine.DirectionalLight"))
  (Variables|Default|SetSky _returnvalue)
  (Utilities|Time|SetTimerbyEvent (delegate Custom|InGameTimer) 1.0 true)
  (if (Variables|Default|GetGameState) :!label _label
    (Utilities|FlowControl|Delay (Variables|Default|GetSpawnSpeed))
    (Game|SpawnActorfromClass "/Game/Blueprints/Blueprints/BP_MatchFallActor.BP_MatchFallActor_C" (Transformation|GetActorTransform (.OutItem (Utilities|Array|Random (Variables|Default|GetFallSpawnPoints)))) "Undefined" "MultiplyWithRoot" 0 0)
    (Audio|PlaySound2D "/Game/StarterContent/Audio/Explosion01.Explosion01" 0.15 1.0 0.0 0 0)
    (Rendering|Components|Light|SetIntensity (Variables|/Script/Engine.Light|GetLightComponent (Variables|Default|GetSky)) (Math|Float|MapRangeClamped (Math|Float|Power (stale Custom|InGameTimer _result) -0.05) 1.0 0.0 (Variables|/Script/Engine.LightComponentBase|GetIntensity (Variables|/Script/Engine.Light|GetLightComponent (Variables|Default|GetSky))) 0.0))
    (goto _label)))

(event EventInit
  (Variables|Default|SetSeconds 3)
  (Pawn|UnPossess (Game|GetPlayerController 0))
  (if (<= (Variables|Default|GetSeconds) 0) :!label _label
    (Default|CallOnFinishedCountdown)
    (CallFunction|OnFinishedCountdownEvent)
    (else
      (Utilities|FlowControl|Delay 1.0)
      (Variables|Default|SetSeconds (- (Variables|Default|GetSeconds) 1))
      (Default|CallOnCountdownUpdate)
      (goto _label))))