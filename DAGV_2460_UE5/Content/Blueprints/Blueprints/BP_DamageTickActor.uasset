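; BP_DamageTickActor is a damage zone that repeatedly hurts a BP_ThirdPersonCharacter standing inside its Box trigger.
; Overlap begin stores the character and starts a looping one-second timer that calls ApplyDamage with DamageValue.
; Overlap end by that character class clears the stored reference and timer, so only one character is tracked at a time.
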(event OnComponentBeginOverlap(Box)
  (params (OverlappedComponent :type Primitive%20Component%20Object%20Reference) (OtherActor :type Actor%20Object%20Reference) (OtherComp :type Primitive%20Component%20Object%20Reference) (OtherBodyIndex :type Integer) (bFromSweep :type Boolean) (SweepResult :type Hit%20Result%20Structure%20%28by%20ref%29))
  (bind _asbp_third_person_character (Utilities|Casting|CastToBP_ThirdPersonCharacter OtherActor))
  (Variables|Default|SetAs%20BP%20Third%20Person%20Character _asbp_third_person_character)
  (bind _returnvalue (Utilities|Time|SetTimerbyEvent (delegate Custom|Damage) 1.0 true))
  (Variables|Default|SetDamageEvent _returnvalue))

(event OnComponentEndOverlap(Box)
  (params (OverlappedComponent :type Primitive%20Component%20Object%20Reference) (OtherActor :type Actor%20Object%20Reference) (OtherComp :type Primitive%20Component%20Object%20Reference) (OtherBodyIndex :type Integer))
  (Utilities|Casting|CastToBP_ThirdPersonCharacter OtherActor)
  (if (and (Utilities|IsValid (Variables|Default|GetAs%20BP%20Third%20Person%20Character)) (Utilities|Time|IsValidTimerHandle (Variables|Default|GetDamageEvent)))
    (Variables|Default|SetAs%20BP%20Third%20Person%20Character 0)
    (Utilities|Time|ClearandInvalidateTimerbyHandle (Variables|Default|GetDamageEvent))
    (Variables|Default|SetDamageEvent "")))

(event Custom|Damage
  (bind _as_bp_third_person_character (Variables|Default|GetAs%20BP%20Third%20Person%20Character))
  (Utilities|IsValid _as_bp_third_person_character
    (:Is%20Valid
      (Game|Damage|ApplyDamage _as_bp_third_person_character (Variables|Default|GetDamageValue) 0 0))))

(fn ConstructionScript)