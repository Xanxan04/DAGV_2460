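; BP_FallActor is a short-lived actor for a matching game that takes a random color when spawned.
; On BeginPlay it caches the GI_MatchingGame instance, applies a random blue, green or red material to its mesh, then sets its lifespan.
; The Box overlap event is empty; disconnected logic for copying the material to the character's sphere and triggering score or reset events by actor type never runs.
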(event EventBeginPlay
  (bind _asgi_matching_game (Utilities|Casting|CastToGI_MatchingGame (Game|GetGameInstance)))
  (Variables|Default|SetAs%20GI%20Matching%20Game _asgi_matching_game)
  (switch int (Math|Random|RandomIntegerinRange 1 3)
    (:1
      (Rendering|Material|SetMaterial (Variables|Default|GetStaticMesh) 0 "/Game/LevelPrototyping/Materials/MI_Solid_Blue.MI_Solid_Blue"))
    (:2
      (Rendering|Material|SetMaterial (Variables|Default|GetStaticMesh) 0 "/Game/Materials/M_Green.M_Green"))
    (:3
      (Rendering|Material|SetMaterial (Variables|Default|GetStaticMesh) 0 "/Game/Materials/M_Red.M_Red")))
  (Actor|SetLifeSpan (Variables|Default|GetLifespan)))

(fn ConstructionScript)

(event OnComponentBeginOverlap(Box)
  (params (OverlappedComponent :type Primitive%20Component%20Object%20Reference) (OtherActor :type Actor%20Object%20Reference) (OtherComp :type Primitive%20Component%20Object%20Reference) (OtherBodyIndex :type Integer) (bFromSweep :type Boolean) (SweepResult :type Hit%20Result%20Structure%20%28by%20ref%29)))