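; BP_MatchActor is a pickup for the matching game that acts as either a Score Actor or a Reset Actor.
; The construction script colors Score Actors randomly blue or green and Reset Actors red.
; On overlap with the third-person character, a Score Actor copies its material to the character's sphere and sends Score to GI_MatchingGame.
; A Reset Actor triggers that game instance's reset event, and both types then destroy themselves.
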(event OnComponentBeginOverlap(Box)
  (params (OverlappedComponent :type Primitive%20Component%20Object%20Reference) (OtherActor :type Actor%20Object%20Reference) (OtherComp :type Primitive%20Component%20Object%20Reference) (OtherBodyIndex :type Integer) (bFromSweep :type Boolean) (SweepResult :type Hit%20Result%20Structure%20%28by%20ref%29))
  (bind _asbp_third_person_character (Utilities|Casting|CastToBP_ThirdPersonCharacter OtherActor))
  (switch Utilities|FlowControl|Switch|SwitchonE_MatchingTypes (Variables|Default|GetActorType)
    (:NewEnumerator0
      (bind _as_gi_matching_game (Variables|Default|GetAs%20GI%20Matching%20Game)
        (:then
          (Rendering|Material|SetMaterial (Variables|/Game/ThirdPerson/Blueprints/BP_ThirdPersonCharacter.BP_ThirdPersonCharacter_C|GetSphere _asbp_third_person_character) 0 (Rendering|Material|GetMaterial (Variables|Default|GetStaticMesh) 0))
          (Default|OnScoreUpdateEvent _as_gi_matching_game (Variables|Default|GetScore)))
        (:else)))
    (:NewEnumerator1
      (bind _as_gi_matching_game_2 (Variables|Default|GetAs%20GI%20Matching%20Game)
        (:then
          (Default|OnResetEvent _as_gi_matching_game_2))
        (:else))))
  (Actor|DestroyActor))

(event EventBeginPlay
  (bind _asgi_matching_game (Utilities|Casting|CastToGI_MatchingGame (Game|GetGameInstance)))
  (Variables|Default|SetAs%20GI%20Matching%20Game _asgi_matching_game))

(fn ConstructionScript
  (switch Utilities|FlowControl|Switch|SwitchonE_MatchingTypes (Variables|Default|GetActorType)
    (:NewEnumerator0
      (switch int (Math|Random|RandomIntegerinRange 1 2)
        (:1
          (Rendering|Material|SetMaterial (Variables|Default|GetStaticMesh) 0 "/Game/LevelPrototyping/Materials/MI_Solid_Blue.MI_Solid_Blue"))
        (:2
          (Rendering|Material|SetMaterial (Variables|Default|GetStaticMesh) 0 "/Game/Materials/M_Green.M_Green"))))
    (:NewEnumerator1
      (Rendering|Material|SetMaterial (Variables|Default|GetStaticMesh) 0 "/Game/Materials/M_Red.M_Red"))))